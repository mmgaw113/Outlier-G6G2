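; Goal actor that ends the game with a win screen when its sphere trigger is overlapped.
; On overlap it resets the player spawn in MyGameInstance to a fixed location, adds WinWidget to the viewport, pauses the game and shows the mouse cursor.
; The overlapping actor is never checked, since the comparison against the player character is unconnected, so any overlapping actor can trigger the win.
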(event `self.Sphere.OnComponentBeginOverlap`
  (params (OverlappedComponent :type "PrimitiveComponent Object Reference") (OtherActor :type "Actor Object Reference") (OtherComp :type "PrimitiveComponent Object Reference") (OtherBodyIndex :type Integer) (bFromSweep :type Boolean) (SweepResult :type "HitResult Structure (by ref)"))
  (bind _asthird_person_character (cast `/Game/ThirdPersonBP/Blueprints/ThirdPersonCharacter` (`GameplayStatics.GetPlayerCharacter` 0)))
  (bind _asmy_game_instance (cast `/Game/Blueprints/MyGameInstance` (`GameplayStatics.GetGameInstance`)))
  (set `/Game/Blueprints/MyGameInstance.PlayerSpawn` (-5125.260254 -4483.150879 224.81485) _asmy_game_instance)
  (bind _returnvalue (`|CreateWidget` "/Game/Widgets/WinWidget.WinWidget_C"))
  (`UserWidget.AddToViewport` _returnvalue 0)
  (`GameplayStatics.SetGamePaused` true)
  (set `PlayerController.bShowMouseCursor` true (`GameplayStatics.GetPlayerController` 0)))

(fn `UserConstructionScript`)